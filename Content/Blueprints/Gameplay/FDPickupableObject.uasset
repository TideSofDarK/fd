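; FDPickupableObject is a pickupable world object that keeps the HUD's nearest-object label updated as overlaps change.
; Begin and end overlap share one path that queries the player character's overlapping FDPickupableObject actors and writes a name to the WNearestObject widget in FDHUD's IngameUI.
; The label shows the last array element's object name, with no distance check, and clears when none overlap.
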(event `self.ReceiveActorEndOverlap`
  (params (OtherActor :type "Actor Object Reference"))
  (bind _overlappingactors (`self.GetOverlappingActors` (`GameplayStatics.GetPlayerCharacter` 0) "FDPickupableObject_C"))
  (for _array_element _overlappingactors :!label _label
    _)
  (bind _asfdhud (cast `/Game/FDHUD` (`PlayerController.GetHUD` (`GameplayStatics.GetPlayerController` 0))))
  (if (== (`KismetArrayLibrary.Array_Length` _overlappingactors) 0)
    (bind _wnearestobject (`/Game/Widgets/WIngameUI.WNearestObject` (`/Game/FDHUD.IngameUI` _asfdhud)))
    (set `/Game/Widgets/WNearestObject.ObjectName` "" _wnearestobject)
    (else
      (set `/Game/Widgets/WNearestObject.ObjectName` (`KismetTextLibrary.Conv_StringToText` (`KismetSystemLibrary.GetObjectName` _array_element)) _wnearestobject))))

(event `self.ReceiveActorBeginOverlap`
  (params (OtherActor :type "Actor Object Reference"))
  (goto _label))

(event `self.ReceiveTick`
  (params (DeltaSeconds :type "Float (single-precision)"))
  (`parent.ReceiveTick` DeltaSeconds))

(fn `UserConstructionScript`
  (`parent.UserConstructionScript`))