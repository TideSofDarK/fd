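; Automatic double sliding door that opens when something overlaps its trigger box.
; Begin overlap plays a sound and runs a timeline that slides two mesh panels apart, mirrored on Y.
; End overlap waits one second, then reverses the timeline if no FDCharacter remains in the box.
; Key-object check and facing-direction helpers are defined, but the door's event graph does not use them.
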(event `self.ReceiveBeginPlay`)

(event `self.ReceiveActorEndOverlap`
  (params (OtherActor :type "Actor Object Reference")))

(event `self.ReceiveActorBeginOverlap`
  (params (OtherActor :type "Actor Object Reference")))

(event `self.BoxComponent.OnComponentBeginOverlap`
  (params (OverlappedComponent :type "PrimitiveComponent Object Reference") (OtherActor :type "Actor Object Reference") (OtherComp :type "PrimitiveComponent Object Reference") (OtherBodyIndex :type Integer) (bFromSweep :type Boolean) (SweepResult :type "HitResult Structure (by ref)"))
  (`GameplayStatics.PlaySoundAtLocation` "/Game/Sounds/SlideDoorA.SlideDoorA" (`SceneComponent.K2_GetComponentLocation` (`self.SceneComponent`)))
  (bind (_direction _slide) (`Timeline|Timeline_0` :!label _label)
    (:`Update`
      (bind _returnvalue (`KismetMathLibrary.MakeVector` 0.0 (+ _slide 100.0) 100.0))
      (`SceneComponent.K2_SetRelativeLocation` (`self.StaticMeshComponent`) (* _returnvalue (1.0 -1.0 1.0)) false false)
      (`SceneComponent.K2_SetRelativeLocation` (`self.StaticMesh2`) _returnvalue false false))))

(event `self.BoxComponent.OnComponentEndOverlap`
  (params (OverlappedComponent :type "PrimitiveComponent Object Reference") (OtherActor :type "Actor Object Reference") (OtherComp :type "PrimitiveComponent Object Reference") (OtherBodyIndex :type Integer))
  (`KismetSystemLibrary.Delay` 1.0)
  (if (not (> (`KismetArrayLibrary.Array_Length` (`PrimitiveComponent.GetOverlappingActors` (`self.BoxComponent`) "/Script/Demo.FDCharacter")) 0))
    (goto _label :!via `Reverse`)))

(fn `CanInteractWith`
  (params (Item :type "FDPickableObject Object Reference"))
  (returns (ReturnValue :type Boolean))
  (return (== Item (`self.KeyObject`))))

(fn `SetLastDirection`
  (params (Actor :type "Actor Object Reference"))
  (set `self.LastDirection` (`KismetMathLibrary.SignOfFloat` (`KismetMathLibrary.Dot_VectorVector` (`self.GetActorForwardVector`) (`self.GetActorForwardVector` Actor)))))

(fn `UserConstructionScript`)