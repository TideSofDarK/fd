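; Lockable swinging door that unlocks when the player uses its KeyObject item, then opens and closes automatically through a trigger volume.
; The interaction delegate, bound on actor overlap, unlocks and opens it with sounds.
; A timeline drives hinge yaw, signed by the dot product of door and actor forward vectors to follow the actor's facing.
; Leaving the trigger reverses the timeline after a delay; direction is re-picked once closed.
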(event `self.ReceiveBeginPlay`)

(event `self.ReceiveActorEndOverlap`
  (params (OtherActor :type "Actor Object Reference")))

(event `self.ReceiveActorBeginOverlap`
  (params (OtherActor :type "Actor Object Reference"))
  (add `self.OnInteractWithItemDelegate` self (delegate `CustomEvent_0`)))

(event `CustomEvent_0` :!signature `self.OnInteractWithItemDelegate`
  (params (Item :type "FDPickableObject Object Reference") (OtherActor :type "FDCharacter Object Reference"))
  (if (not (`self.Unlocked`))
    (set `self.Unlocked` true)
    (`self.SetLastDirection` OtherActor)
    (`GameplayStatics.PlaySoundAtLocation` "/Game/Sounds/DoorUnlockA.DoorUnlockA" (`self.K2_GetActorLocation` self))
    ;[1 1 1] Collision
    (set `self.NearDoor` true :!label _label)
    (`GameplayStatics.PlaySoundAtLocation` "/Game/Sounds/DoorCreakA.DoorCreakA" (`self.K2_GetActorLocation` self))
    (bind (_direction _door) (`Timeline|Timeline_0` :!label _label_2)
      (:`Update`
        (`SceneComponent.K2_SetRelativeRotation` (`self.SceneComponent`) (`KismetMathLibrary.MakeRotator` 0.0 0.0 (* (`self.LastDirection`) _door)) false false))
      (:`Finished`
        (set `self.Direction` _direction)))))

(event `self.DoorTrigger.OnComponentBeginOverlap`
  (params (OverlappedComponent :type "PrimitiveComponent Object Reference") (OtherActor :type "Actor Object Reference") (OtherComp :type "PrimitiveComponent Object Reference") (OtherBodyIndex :type Integer) (bFromSweep :type Boolean) (SweepResult :type "HitResult Structure (by ref)"))
  ;[1 1 1] Collision
  (if (`self.Unlocked`)
    (if (`self.NearDoor`)
      _
      (elif (or (`|EnumEquality` (`self.Direction`) "Backward") (== (`self.LastDirection`) 0.0))
        (`self.SetLastDirection` OtherActor)
        (goto _label)
        (else
          (goto _label))))))

(event `self.DoorTrigger.OnComponentEndOverlap`
  (params (OverlappedComponent :type "PrimitiveComponent Object Reference") (OtherActor :type "Actor Object Reference") (OtherComp :type "PrimitiveComponent Object Reference") (OtherBodyIndex :type Integer))
  ;[1 1 1] Collision
  (if (`self.Unlocked`)
    (`KismetSystemLibrary.Delay` 3.0)
    (set `self.NearDoor` false)
    (goto _label_2 :!via `Reverse`)))

(fn `CanInteractWith`
  (params (Item :type "FDPickableObject Object Reference"))
  (returns (ReturnValue :type Boolean))
  (return (== Item (`self.KeyObject`))))

(fn `SetLastDirection`
  (params (Actor :type "Actor Object Reference"))
  (set `self.LastDirection` (`KismetMathLibrary.SignOfFloat` (`KismetMathLibrary.Dot_VectorVector` (`self.GetActorForwardVector`) (`self.GetActorForwardVector` Actor)))))

(fn `UserConstructionScript`)