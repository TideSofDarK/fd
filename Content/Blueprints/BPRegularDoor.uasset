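; A regular swinging door actor that opens automatically when an actor overlaps it and closes three seconds after the overlap ends.
; On overlap, the dot product of the door's and visitor's forward vectors sets the swing sign, so it opens along the visitor's facing.
; A timeline drives the scene component's relative yaw, and the sign updates only when the door last finished reversing or none is set.
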(event `self.ReceiveBeginPlay`
  (`self.EnableInput` null))

(event `self.ReceiveActorBeginOverlap`
  (params (OtherActor :type "Actor Object Reference"))
  ;[1 1 1] Collision
  (if (not (`self.NearDoor`))
    (if (or (`|EnumEquality` (`self.Direction`) "Backward") (== (`self.LastDirection`) 0.0))
      (set `self.LastDirection` (`KismetMathLibrary.SignOfFloat` (`KismetMathLibrary.Dot_VectorVector` (`self.GetActorForwardVector`) (`self.GetActorForwardVector` OtherActor)))))
    (set `self.NearDoor` true)
    (bind (_direction _door) (`Timeline|Timeline_0` :!label _label)
      (:`Update`
        (`SceneComponent.K2_SetRelativeRotation` (`self.Scene`) (`KismetMathLibrary.MakeRotator` 0.0 0.0 (* (`self.LastDirection`) _door)) false false))
      (:`Finished`
        (set `self.Direction` _direction)))))

(event `self.ReceiveActorEndOverlap`
  (params (OtherActor :type "Actor Object Reference"))
  ;[1 1 1] Collision
  (`KismetSystemLibrary.Delay` 3.0)
  (set `self.NearDoor` false)
  (goto _label :!via `Reverse`))

(fn `UserConstructionScript`)